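; Moving ball Blueprint that records its timestamped movement history and can be reset to its start location.
; ObjectTimer loops on itself through a Delay, advancing the clock while RecordTransform appends time, location and rotation whenever the location changes.
; Enter stops the timer, saves the end time, zeroes the clock and teleports the ball back to its initial location.
; The recorded list is never replayed here, despite the Playback label.
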(event `ObjectTimer`
  (bind _timervalue (`self.TimerValue`))
  ;[1 0.1365 0.1365] Timer
  (`self.RecordTransform`)
  (if (`self.TimerActivated`)
    (`KismetSystemLibrary.Delay` _timervalue)
    (bind _output_get (set `self.CurrentTime` (+ _timervalue (`self.CurrentTime`))))
    ;;[1 1 1] VisibleTimer
    (`KismetSystemLibrary.PrintString` (`KismetStringLibrary.Conv_DoubleToString` _output_get) true true (struct :`G` 0.66 :`B` 1.0 :`A` 1.0) (`self.TimerValue`))
    (`self.ObjectTimer`)))

(event `self.ReceiveBeginPlay`
  (bind (_returnvalue_location _returnvalue_rotation) (`KismetMathLibrary.BreakTransform` (`self.GetTransform`)))
  (bind _output_get (set `self.InitLocation` _returnvalue_location))
  (bind _output_get_2 (set `self.LastLocation` _output_get))
  (bind _output_get_3 (set `self.TimingTransformStruct` (make `/Game/Timing/Timing_Transform_Struct` 0.0 _output_get_2 _returnvalue_rotation)))
  (`KismetArrayLibrary.Array_Add` (`self.TimingTransformStructList`) _output_get_3))

(event `Key|Enter`
  (params (Key :type "Key Structure"))
  ;[0.4956 0.4698 1] Playback
  (:`Pressed`
    (`KismetSystemLibrary.PrintString` "Timer Stopped")
    (set `self.TimerActivated` false)
    (bind _output_get (set `self.TimerEnd` (`self.CurrentTime`)))
    (set `self.CurrentTime` 0.0)
    (`self.K2_SetActorLocation` (`self.InitLocation`) false true)))

(fn `RecordTransform`
  (bind (_returnvalue_location _returnvalue_rotation) (`KismetMathLibrary.BreakTransform` (`self.GetTransform`)))
  (if (== _returnvalue_location (`self.LastLocation`))
    (return)
    (else
      (bind _output_get (set `self.TimingTransformStruct` (make `/Game/Timing/Timing_Transform_Struct` (`self.CurrentTime`) _returnvalue_location _returnvalue_rotation)))
      (`KismetArrayLibrary.Array_Add` (`self.TimingTransformStructList`) _output_get)
      (set `self.LastLocation` _returnvalue_location)
      (return))))

(fn `TimerEvent`)

(fn `UserConstructionScript`)